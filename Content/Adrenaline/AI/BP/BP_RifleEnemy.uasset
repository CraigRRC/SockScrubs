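; Rifle-wielding enemy built on BaseEnemy that shoots projectiles.
; On BeginPlay it disables actor tick on its AI controller.
; Its Fire override spawns a BP_RifleProjectile at the spawn point and plays a gunshot with slightly randomized pitch.
; The construction script snaps the gun mesh to the Weapon socket, and the head hitbox and health widget to the shared HeadHitbox socket.
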(event EventBeginPlay
  (bind _asaicontroller (Utilities|Casting|CastToAIController (Pawn|GetController)))
  (Actor|Tick|SetActorTickEnabled _asaicontroller))

(event Collision|EventActorBeginOverlap
  (params (OtherActor :type Actor%20Object%20Reference)))

(event EventFire
  ;[1 1 1] Override of the Fire Function called from BaseEnemy
  (Game|SpawnActorfromClass "/Game/Adrenaline/AI/Projectiles/BP_RifleProjectile.BP_RifleProjectile_C" (Transformation|GetWorldTransform (Variables|Default|GetProjectileSpawnPoint)) "AlwaysSpawn" "MultiplyWithRoot" 0 0)
  (Audio|PlaySoundatLocation "/Game/Adrenaline/Audio/CUE/Guns_shot_Cue.Guns_shot_Cue" (Transformation|GetActorLocation) "0, 0, 0" 1.0 (Math|Random|RandomFloatinRange 0.8 1.0) 0.0 "/Game/Adrenaline/Audio/Attenuation/EnemyGunfire.EnemyGunfire" 0 0 0))

(fn ConstructionScript
  (bind _enemymesh (Variables|Default|GetEnemyMesh))
  (Transformation|AttachComponentToComponent (Variables|Default|GetTempGunMesh) (Variables|Default|GetEnemyMesh) "Weapon" "SnapToTarget" "SnapToTarget" "KeepWorld" true)
  (Transformation|AttachComponentToComponent (Variables|Default|GetHeadHitbox) _enemymesh "HeadHitbox" "SnapToTarget" "SnapToTarget" "KeepRelative" true)
  (Transformation|AttachComponentToComponent (Variables|Default|GetHealthWidgetComponent) _enemymesh "HeadHitbox" "SnapToTarget" "SnapToTarget" "KeepRelative" true))