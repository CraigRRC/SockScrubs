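; Temporary ranged enemy that faces the player within a debug-drawn radius, shows its HP widget and fires projectiles on a Delay/DoOnce cooldown.
; TakeDamage either stuns it or subtracts health, feeding a percentage that Tick pushes to the widget.
; A first stun or death drops a physics rifle pickup, permanently disabling firing and hiding Mesh.
; Death also broadcasts Died with an adrenaline build amount and expires the actor.
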(event EventBeginPlay
  (bind _hp_percent (CallFunction|ConvertHPtoPercent (Variables|Default|GetHealth)))
  (Variables|Default|SetHPPercent _hp_percent)
  (bind _aswbp_enemy_hp (Utilities|Casting|CastToWBP_EnemyHP (UserInterface|GetWidget (Variables|Default|GetHP))))
  (Variables|Default|SetWBP%20Enemy%20HP _aswbp_enemy_hp))

(event EventTakeDamage
  (params (DamageValue :type Float%20%28double-precision%29) (Stun :type Boolean))
  (if Stun
    (Class|PrimitiveComponent|SetConstraintMode (Variables|Collision|GetCapsuleComponent) "None")
    (if (not (Variables|Default|GetStun))
      (Variables|Default|SetStun true)
      (if (not (Variables|Default|GetDroppedWeapon))
        (bind _returnvalue (Game|SpawnActorfromClass "/Game/FirstPerson/Blueprints/BP_Pickup_Rifle.BP_Pickup_Rifle_C" (Transformation|GetActorTransform) "Undefined" "MultiplyWithRoot" 0 0))
        (Variables|Default|SetDroppedWeapon true)
        (Collision|SetCollisionResponsetoChannel (Variables|/Game/FirstPerson/Blueprints/BP_Pickup_Rifle.BP_Pickup_Rifle_C|GetSphereCollision _returnvalue) "ECC_GameTraceChannel1" "ECR_Ignore")
        (Physics|SetSimulatePhysics (Variables|/Game/FirstPerson/Blueprints/BP_Pickup_Rifle.BP_Pickup_Rifle_C|GetSkeletalMesh _returnvalue) true)
        (Collision|SetCollisionResponsetoChannel (Variables|/Game/FirstPerson/Blueprints/BP_Pickup_Rifle.BP_Pickup_Rifle_C|GetStun _returnvalue) "ECC_Pawn" "ECR_Ignore")
        (Utilities|FlowControl|Delay 5.0)
        (Variables|Default|SetStun false)
        (Variables|Default|SetCustomTimeDilation 1.0)))
    (elif (not (<= (Variables|Default|GetHealth) 0.0))
      (Variables|Default|SetHealth (- (Variables|Default|GetHealth) DamageValue))
      (bind _hp_percent (CallFunction|ConvertHPtoPercent (Variables|Default|GetHealth)))
      (Variables|Default|SetHPPercent _hp_percent)
      (if (<= (Variables|Default|GetHealth) 0.0)
        (Default|CallDied (Variables|Default|GetAdren%20Build%20Amount))
        (Actor|SetLifeSpan 0.1)
        (Utilities|FlowControl|DoOnce false
          (:Completed
            (Collision|SetCollisionEnabled (Variables|Collision|GetCapsuleComponent) "NoCollision")
            (if (not (Variables|Default|GetDroppedWeapon))
              (bind _returnvalue_2 (Game|SpawnActorfromClass "/Game/FirstPerson/Blueprints/BP_Pickup_Rifle.BP_Pickup_Rifle_C" (Transformation|GetActorTransform) "Undefined" "MultiplyWithRoot" 0 0))
              (Variables|Default|SetDroppedWeapon true)
              (Collision|SetCollisionResponsetoChannel (Variables|/Game/FirstPerson/Blueprints/BP_Pickup_Rifle.BP_Pickup_Rifle_C|GetSphereCollision _returnvalue_2) "ECC_GameTraceChannel1" "ECR_Ignore")
              (Physics|SetSimulatePhysics (Variables|/Game/FirstPerson/Blueprints/BP_Pickup_Rifle.BP_Pickup_Rifle_C|GetSkeletalMesh _returnvalue_2) true)
              (Collision|SetCollisionResponsetoChannel (Variables|/Game/FirstPerson/Blueprints/BP_Pickup_Rifle.BP_Pickup_Rifle_C|GetStun _returnvalue_2) "ECC_Pawn" "ECR_Ignore"))))))))

(event EventTick
  (params (DeltaSeconds :type Float%20%28single-precision%29))
  (bind _returnvalue (Math|Random|RandomFloatinRange 0.5 1.0))
  (bind _hp (Variables|Default|GetHP))
  (Utilities|FlowControl|Sequence
    (:then_0
      (Rendering|Debug|DrawDebugSphere (Transformation|GetActorLocation) (Variables|Default|GetRadius) 12 "(R=1.000000,G=0.103049,B=0.000000,A=1.000000)" 0.0))
    (:then_1
      (Variables|Default|SetCanFire (not (Variables|Default|GetDroppedWeapon)))
      (if (Variables|Default|GetDroppedWeapon)
        (Rendering|SetVisibility (Variables|Character|GetMesh) false false)))
    (:then_2
      (if (Variables|Default|GetStun)
        (Development|PrintString "Stunned!" true true "(R=0.000000,G=0.660000,B=1.000000,A=1.000000)" 1.0)
        (elif (<= (Math|Vector|VectorLength (- (Transformation|GetActorLocation (Game|Player|GetPlayerPawn 0)) (Transformation|GetActorLocation))) (Variables|Default|GetRadius))
          (Rendering|SetVisibility _hp true false)
          (Transformation|SetActorRotation (Math|Rotator|FindLookatRotation (Transformation|GetActorLocation) (Transformation|GetActorLocation (Game|Player|GetPlayerPawn 0))))
          (Utilities|FlowControl|Delay 0.2)
          (Utilities|FlowControl|DoOnce false :!label _label
            (:Completed
              (if (Variables|Default|GetCanFire)
                (Game|SpawnActorfromClass "/Game/FirstPerson/Blueprints/BP_EnemyProjectile.BP_EnemyProjectile_C" (Transformation|GetWorldTransform (Variables|Default|GetProjectileSpawn)) "Undefined" "MultiplyWithRoot" 0 0)
                (Audio|PlaySoundatLocation "/Game/StarterContent/Audio/Explosion_Cue.Explosion_Cue" (Transformation|GetActorLocation) "0, 0, 0" _returnvalue _returnvalue 0.0 "/Game/Adrenaline/Audio/EnemyGunfire.EnemyGunfire" 0 0 0)
                (Utilities|FlowControl|Delay 1.5)
                (goto _label Reset))))
          (else
            (Rendering|SetVisibility _hp false false)))))
    (:then_3
      (Utilities|IsValid (Variables|Default|GetWBP%20Enemy%20HP)
        (:Is%20Valid
          (Variables|/Game/Adrenaline/UI/WBP_EnemyHP.WBP_EnemyHP_C|SetHealthPercent (Variables|Default|GetWBP%20Enemy%20HP) (Variables|Default|GetHPPercent)))))))

(event Collision|EventActorBeginOverlap
  (params (OtherActor :type Actor%20Object%20Reference)))

(fn ConstructionScript)

(fn ConvertHPtoPercent
  (params (HP%20Float :type Float%20%28double-precision%29))
  (return (Math|Float|SafeDivide HP%20Float (Variables|Default|GetMaxHp))))