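; BP_Building is a PCG-driven building actor with an adjustable floor count.
; Its construction script feeds two vector parameters into the PCG component's graph instance, and it has no runtime logic.
; "Floors" carries a height of 400 units per floor above the first, clamped to at least 1.
; "FloorCopyOffset" carries the actor's location with X and Z swapped and negated.
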(event EventBeginPlay)

(event Collision|EventActorBeginOverlap
  (params (OtherActor :type Actor%20Object%20Reference)))

(event EventTick
  (params (DeltaSeconds :type Float%20%28single-precision%29)))

(fn ConstructionScript
  (bind _returnvalue (Transformation|GetActorLocation))
  (bind _pcg (Variables|Default|GetPCG))
  (bind _graphinstance (Variables|/Script/PCG.PCGComponent|GetGraphInstance _pcg))
  (Effects|Components|ParticleSystem|SetVectorParameter _graphinstance "Floors" (Math|Vector|MakeVector 0.0 0.0 (Math|Conversions|ToFloat(Integer) (Math|Integer|Max(Integer) (* 400 (- (Variables|Default|GetFloors) 1)) 1))))
  (Effects|Components|ParticleSystem|SetVectorParameter _graphinstance "FloorCopyOffset" (Math|Vector|MakeVector (* (.z _returnvalue) -1.0) (.y _returnvalue) (* (.x _returnvalue) -1.0))))